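; BP_LogisticsManager is the central tracker for a parcel logistics simulation, holding parcel counts, system status, event logs and ID generation.
; Entry and processing calls update in-system, total and per-destination counts, while a 10-second timer derives per-minute throughput with a six-sample history.
; Scans feed a queue count that switches overload status using separate overload and recovery thresholds.
; Dispatchers broadcast data, status and log changes, and a toggle sets ID visibility on all parcels.
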(event `self.ReceiveBeginPlay`
  ; Throughput 계산. 10초 갱신
  (`KismetSystemLibrary.K2_SetTimer` null "CalculateThroughput" 10.0 true))

(fn `AddEventLog`
  (params (LogType :type "/Game/Data/Enum/E_LogType Enum" :default "NewEnumerator0") (Source :type String) (EventMessage :type String) (ParcelID :type String) (Destination :type "/Game/Data/Enum/E_Destination Enum" :default "NewEnumerator0"))
  (bind (_returnvalue_year _returnvalue_month _returnvalue_day _returnvalue_hour _returnvalue_minute _returnvalue_second) (`KismetMathLibrary.BreakDateTime` (`KismetMathLibrary.Now`)))
  ; 새로운 로그 데이터 로그 배열에 저장
  (`KismetArrayLibrary.Array_Add` (`self.EventLogs`) (make `/Game/Data/Structure/ST_EventLog` (`KismetTextLibrary.Conv_TextToString` (`|FormatText` "{Hour}:{Min}:{Sec}" _returnvalue_hour _returnvalue_minute _returnvalue_second)) LogType Source EventMessage ParcelID Destination))
  ;; 로그 변경 방송
  (`self.OnEventLogChanged`))

(fn `CalculateThroughput`
  (bind _throughputhistory (`self.ThroughputHistory`))
  ; 흐름량 계산 함수. 10초당 갱신 + Throughput History 배열도 관리. 길이가 6 초과면 가장 앞에 정보 삭제
  (bind _output_get (set `self.Throughput` (* (`self.ProcessedInWindow`) 6)))
  (`KismetArrayLibrary.Array_Add` _throughputhistory (`KismetMathLibrary.Conv_IntToDouble` _output_get))
  (if (> (`KismetArrayLibrary.Array_Length` _throughputhistory) 6)
    (`KismetArrayLibrary.Array_Remove` (`self.ThroughputHistory`)))
  (set `self.ProcessedInWindow` 0)
  (`self.OnDataChanged` (`self.InSystem`) (`self.TotalProcessed`) _output_get))

(fn `GenerateParcelID`
  (returns (ParcelID :type Text))
  (set `self.GeneratedID` (`|FormatText` "P-{id}" (`KismetTextLibrary.Conv_IntToText` (`self.NextParcelID`) false false 5)))
  (`/Engine/EditorBlueprintResources/StandardMacros.IncrementInt` (`self.NextParcelID`)
    (:`  `
      (return (`self.GeneratedID`)))))

(fn `ParcelEnteredSystem`
  ; Parcel 생성시 insystem +1, 콜까지 해주는 함수
  (bind _result (`/Engine/EditorBlueprintResources/StandardMacros.IncrementInt` (`self.InSystem`))
    (:`  `
      (`self.OnDataChanged` _result (`self.TotalProcessed`) (`self.Throughput`)))))

(fn `ParcelProcessed`
  (params (`Parcel Destination` :type "/Game/Data/Enum/E_Destination Enum" :default "NewEnumerator0"))
  ; 박스 이탈시 insys-1, total pro +1, 콜까지 해주는 함수
  (`|ExecutionSequence`
    (:`then_0`
      (`/Engine/EditorBlueprintResources/StandardMacros.DecrementInt` (`self.InSystem`)
        (:`  `
          (`/Engine/EditorBlueprintResources/StandardMacros.IncrementInt` (`self.TotalProcessed`)
            (:`  `
              (`/Engine/EditorBlueprintResources/StandardMacros.IncrementInt` (`self.ProcessedInWindow`)))))))
    (:`then_1`
      ;; 목적지에 따른 처리량 증가
      (switch `/Game/Data/Enum/E_Destination` `Parcel Destination`
        (:`NewEnumerator0`
          (`/Engine/EditorBlueprintResources/StandardMacros.IncrementInt` (`self.OkcheonProcessed`)
            (:`  `
              _)))
        (:`NewEnumerator1`
          (`/Engine/EditorBlueprintResources/StandardMacros.IncrementInt` (`self.DaejeonProcessed`)
            (:`  `
              _)))
        (:`NewEnumerator2`
          (`/Engine/EditorBlueprintResources/StandardMacros.IncrementInt` (`self.GonjiamProcessed`)
            (:`  `
              _))))
      (`self.OnDataChanged` (`self.InSystem`) (`self.TotalProcessed`) (`self.Throughput`)))))

(fn `ParcelScanned`
  (params (Parcel :type "/Game/Blueprint/Parcel/BP_Parcel Object Reference"))
  (bind _scannedparcel (`self.ScannedParcel`))
  (`KismetArrayLibrary.Array_AddUnique` _scannedparcel Parcel)
  (`self.UpdateSystemStatus` (`KismetArrayLibrary.Array_Length` _scannedparcel)))

(fn `SetShowParcelID`
  (params (bShow :type Boolean))
  (set `self.bShowParcelID` bShow)
  (bind _outactors (`GameplayStatics.GetAllActorsOfClass` "/Game/Blueprint/Parcel/BP_Parcel.BP_Parcel_C"))
  (for _array_element _outactors
    (bind _asbp_parcel (cast `/Game/Blueprint/Parcel/BP_Parcel` _array_element))
    (`/Game/Blueprint/Parcel/BP_Parcel.SetParcelIDVisible` _asbp_parcel bShow)))

(fn `UpdateSystemStatus`
  (params (QueueCount :type Integer))
  ; Queue의 길이를 통해 현재 상태를 확인하는 함수, 상태가 바뀌면 바뀐 상태를 브로드 캐스팅
  (if (and (>= QueueCount (`self.OverloadThreshold`)) (`|EnumInequality` (`self.SystemStatus`) "NewEnumerator2"))
    ;; 한계점을 넘으면 + 이전 상태가 오버로드가 아니라면 오버로드로 바꿈
    (bind _output_get (set `self.SystemStatus` "NewEnumerator2"))
    (`self.OnSystemStatusChanged` _output_get)
    (elif (and (<= (`local.QueueCount`) (`self.RecoveryThreshold`)) (`|EnumEquality` (`self.SystemStatus`) "NewEnumerator2"))
      (bind _output_get_2 (set `self.SystemStatus` "NewEnumerator1"))
      (`self.OnSystemStatusChanged` _output_get_2))))

(fn `UserConstructionScript`)