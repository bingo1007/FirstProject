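; Conveyor sorter machine that routes scanned parcels by destination in a logistics simulation.
; It handles one parcel at a time, claiming the first in the LogisticsManager's scanned list that overlaps SorterArea, then moving it each Tick along the Up, Straight or Down arrow.
; On exit, it removes that parcel, sends a SORTED HTTP event, updates system status and takes the next.
; Clicking it reports the selection to the player controller.
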(event `self.ReceiveBeginPlay`
  ; 상태 체크 함수를 사용하기 위해 LogisticsManager 캐싱
  (bind _returnvalue (`GameplayStatics.GetActorOfClass` "/Game/Blueprint/Core/BP_LogisticsManager.BP_LogisticsManager_C"))
  (bind _asbp_logistics_manager (cast `/Game/Blueprint/Core/BP_LogisticsManager` _returnvalue))
  (set `self.LogisticsManagerRef` _asbp_logistics_manager))

(event `self.SorterArea.OnComponentBeginOverlap`
  (params (OverlappedComponent :type "PrimitiveComponent Object Reference") (OtherActor :type "Actor Object Reference") (OtherComp :type "PrimitiveComponent Object Reference") (OtherBodyIndex :type Integer) (bFromSweep :type Boolean) (SweepResult :type "HitResult Structure (by ref)"))
  ; Sorter에 들어왔다면 들어온 상태 저장
  (bind _asbp_parcel (cast `/Game/Blueprint/Parcel/BP_Parcel` OtherActor))
  (set `/Game/Blueprint/Parcel/BP_Parcel.bEnterConveyor` false _asbp_parcel)
  (set `/Game/Blueprint/Parcel/BP_Parcel.bEnterSorter` true _asbp_parcel)
  (`self.TryProcessNextParcel`))

(event `self.SorterArea.OnComponentEndOverlap`
  (params (OverlappedComponent :type "PrimitiveComponent Object Reference") (OtherActor :type "Actor Object Reference") (OtherComp :type "PrimitiveComponent Object Reference") (OtherBodyIndex :type Integer))
  (bind _logisticsmanagerref (`self.LogisticsManagerRef`))
  (bind _scannedparcel (`/Game/Blueprint/Core/BP_LogisticsManager.ScannedParcel` (`self.LogisticsManagerRef`)))
  ; Sorter에서 나갔다면 Sensor에서 인지한 Parcels 중 나간 Parcel 삭제
  (bind _asbp_parcel (cast `/Game/Blueprint/Parcel/BP_Parcel` OtherActor))
  (if (== OtherActor (`self.CurrentParcel`))
    (`KismetArrayLibrary.Array_RemoveItem` _scannedparcel (`self.CurrentParcel`))
    (`LogisticsHttpSubsystem.SendParcelEvent` (subsystem `LogisticsHttpSubsystem`) (`KismetStringLibrary.Conv_StringToInt` (`KismetStringLibrary.RightChop` (`/Game/Blueprint/Parcel/BP_Parcel.ParcelID` _asbp_parcel) 2)) "SORTED" (`|GetEnumeratorNameAsString` (`/Game/Blueprint/Parcel/BP_Parcel.Destination` _asbp_parcel)))
    ;; 삭제 후 상태 체크
    (`/Engine/EditorBlueprintResources/StandardMacros.IsValid` _logisticsmanagerref
      (:`Is Valid`
        (`/Game/Blueprint/Core/BP_LogisticsManager.UpdateSystemStatus` _logisticsmanagerref (`KismetArrayLibrary.Array_Length` _scannedparcel))
        (set `self.CurrentParcel` null)
        (`self.TryProcessNextParcel`)))))

(event `self.ReceiveTick`
  (params (DeltaSeconds :type "Float (single-precision)"))
  ; 방향 결정 및 이동
  (`/Engine/EditorBlueprintResources/StandardMacros.IsValid` (`self.CurrentParcel`)
    (:`Is Valid`
      (switch `/Game/Data/Enum/E_SortDirection` (`self.SortDirection`)
        (:`NewEnumerator0`
          (`self.K2_SetActorLocation` (`self.CurrentParcel`) (+ (* (`self.MoveSpeed`) (`GameplayStatics.GetWorldDeltaSeconds`) (`SceneComponent.GetForwardVector` (`self.UpArrow`))) (`self.K2_GetActorLocation` (`self.CurrentParcel`))) false false))
        (:`NewEnumerator1`
          (`self.K2_SetActorLocation` (`self.CurrentParcel`) (+ (* (`self.MoveSpeed`) (`GameplayStatics.GetWorldDeltaSeconds`) (`SceneComponent.GetForwardVector` (`self.StraightArrow`))) (`self.K2_GetActorLocation` (`self.CurrentParcel`))) false false))
        (:`NewEnumerator2`
          (`self.K2_SetActorLocation` (`self.CurrentParcel`) (+ (* (`self.MoveSpeed`) (`GameplayStatics.GetWorldDeltaSeconds`) (`SceneComponent.GetForwardVector` (`self.DownArrow`))) (`self.K2_GetActorLocation` (`self.CurrentParcel`))) false false))))))

(event `self.Cube.OnClicked`
  (params (TouchedComponent :type "PrimitiveComponent Object Reference") (ButtonPressed :type "Key Structure"))
  ; 클릭시 Sorter 객체 컨트롤러에 전달
  (bind _asbp_player_contoller (cast `/Game/Blueprint/Core/BP_PlayerContoller` (`GameplayStatics.GetPlayerController` 0)))
  (`/Game/Blueprint/Core/BP_PlayerContoller.OnEquipmentSelected` _asbp_player_contoller self)
  (`KismetSystemLibrary.PrintString` "전달완료"))

(fn `TryProcessNextParcel`
  (bind _currentparcel (`self.CurrentParcel`))
  ; 조건 1 : 현재 처리하고 있는 택배가 있나?
  (`/Engine/EditorBlueprintResources/StandardMacros.IsValid` (`self.CurrentParcel`)
    (:`Is Not Valid`
      ; 조건 2 : 현재 큐에 처리 할 택배가 있는가?
      (if (not (`KismetArrayLibrary.Array_IsEmpty` (`/Game/Blueprint/Core/BP_LogisticsManager.ScannedParcel` (`self.LogisticsManagerRef`))))
        ; 조건 3 : 현재 큐의 요소가 감지 구역에 들어 왔는가?
        (for _array_element (`/Game/Blueprint/Core/BP_LogisticsManager.ScannedParcel` (`self.LogisticsManagerRef`))
          (if (`PrimitiveComponent.IsOverlappingActor` (`self.SorterArea`) _array_element)
            ; 모든 조건에 부합하다면 해당 택배를 처리할 택배로 판단, 목적지를 분류한다. + 로그 추가까지
            (bind _output_get (set `self.CurrentParcel` _array_element))
            (switch `/Game/Data/Enum/E_Destination` (`/Game/Blueprint/Parcel/BP_Parcel.Destination` _output_get)
              (:`NewEnumerator0`
                (set `self.SortDirection` "NewEnumerator0")
                (`self.OnSorterStateChanged` self))
              (:`NewEnumerator1`
                (set `self.SortDirection` "NewEnumerator1")
                (`self.OnSorterStateChanged` self))
              (:`NewEnumerator2`
                (set `self.SortDirection` "NewEnumerator2")
                (`self.OnSorterStateChanged` self)))
            (`/Game/Blueprint/Core/BP_LogisticsManager.AddEventLog` (`self.LogisticsManagerRef`) "NewEnumerator0" "Sorter-01" "Parcel Sorted" (`/Game/Blueprint/Parcel/BP_Parcel.ParcelID` _currentparcel) (`/Game/Blueprint/Parcel/BP_Parcel.Destination` _currentparcel))
            (break)))))))

(fn `UserConstructionScript`)