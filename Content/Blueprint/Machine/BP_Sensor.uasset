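; BP_Sensor is a scanner in the logistics simulation that registers parcels as they enter its overlap sphere.
; On BeginPlay it caches the BP_LogisticsManager found in the level.
; Each BP_Parcel overlap calls ParcelScanned on the manager, sends a SCANNED event through LogisticsHttpSubsystem, and logs the scan under the sensor's ID.
; The HTTP event uses a numeric ID made by trimming two leading characters from the parcel's string ID.
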(event `self.ReceiveBeginPlay`
  ; 상태 함수를 사용하기 위해 LogisticsManager 객체 캐싱
  (bind _returnvalue (`GameplayStatics.GetActorOfClass` "/Game/Blueprint/Core/BP_LogisticsManager.BP_LogisticsManager_C"))
  (bind _asbp_logistics_manager (cast `/Game/Blueprint/Core/BP_LogisticsManager` _returnvalue))
  (set `self.LogisticsManagerRef` _asbp_logistics_manager))

(event `self.Sphere1.OnComponentBeginOverlap`
  (params (OverlappedComponent :type "PrimitiveComponent Object Reference") (OtherActor :type "Actor Object Reference") (OtherComp :type "PrimitiveComponent Object Reference") (OtherBodyIndex :type Integer) (bFromSweep :type Boolean) (SweepResult :type "HitResult Structure (by ref)"))
  (bind _logisticsmanagerref (`self.LogisticsManagerRef`))
  ; 센서에 닿을때마다 택배 큐에 삽입
  (bind _asbp_parcel (cast `/Game/Blueprint/Parcel/BP_Parcel` OtherActor))
  (`/Engine/EditorBlueprintResources/StandardMacros.IsValid` _logisticsmanagerref
    (:`Is Valid`
      (`/Game/Blueprint/Core/BP_LogisticsManager.ParcelScanned` _logisticsmanagerref _asbp_parcel)
      (bind _parcelid (`/Game/Blueprint/Parcel/BP_Parcel.ParcelID` _asbp_parcel))
      (bind _destination (`/Game/Blueprint/Parcel/BP_Parcel.Destination` _asbp_parcel))
      (`LogisticsHttpSubsystem.SendParcelEvent` (subsystem `LogisticsHttpSubsystem`) (`KismetStringLibrary.Conv_StringToInt` (`KismetStringLibrary.RightChop` _parcelid 2)) "SCANNED" (`|GetEnumeratorNameAsString` _destination))
      (`/Game/Blueprint/Core/BP_LogisticsManager.AddEventLog` (`self.LogisticsManagerRef`) "NewEnumerator0" (`self.SensorID`) "Parcel Scanned" _parcelid _destination))))

(fn `UserConstructionScript`)