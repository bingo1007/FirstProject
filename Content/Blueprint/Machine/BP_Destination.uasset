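; BP_Destination is a logistics drop-off point that receives parcels routed to its destination.
; Its box overlap ignores parcels bound elsewhere; matching ones increment a count, get reported to BP_LogisticsManager as processed and logged as arrived, then are destroyed.
; The manager is found by class on BeginPlay, and a full count rolls over into a pallet tally and resets.
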(event `self.ReceiveBeginPlay`
  (bind _returnvalue (`GameplayStatics.GetActorOfClass` "/Game/Blueprint/Core/BP_LogisticsManager.BP_LogisticsManager_C"))
  (bind _asbp_logistics_manager (cast `/Game/Blueprint/Core/BP_LogisticsManager` _returnvalue))
  (set `self.LogisticsManagerRef` _asbp_logistics_manager))

(event `self.Box.OnComponentBeginOverlap`
  (params (OverlappedComponent :type "PrimitiveComponent Object Reference") (OtherActor :type "Actor Object Reference") (OtherComp :type "PrimitiveComponent Object Reference") (OtherBodyIndex :type Integer) (bFromSweep :type Boolean) (SweepResult :type "HitResult Structure (by ref)"))
  (bind _asbp_parcel (cast `/Game/Blueprint/Parcel/BP_Parcel` OtherActor))
  (bind _destination (`/Game/Blueprint/Parcel/BP_Parcel.Destination` _asbp_parcel))
  (if (`|EnumEquality` _destination (`self.Destination`))
    (`/Engine/EditorBlueprintResources/StandardMacros.IncrementInt` (`self.CurrentCount`)
      (:`  `
        ; 빠져 나갔으면 sys -1, total +1
        (`/Game/Blueprint/Core/BP_LogisticsManager.ParcelProcessed` (`self.LogisticsManagerRef`) _destination)
        (`/Game/Blueprint/Core/BP_LogisticsManager.AddEventLog` (`self.LogisticsManagerRef`) "NewEnumerator0" "Destination" "Parcel Arrived" (`/Game/Blueprint/Parcel/BP_Parcel.ParcelID` _asbp_parcel) _destination)
        (`self.CheckPalletFull`)
        (`self.K2_DestroyActor` _asbp_parcel)))))

(fn `CheckPalletFull`
  (if (>= (`self.CurrentCount`) (`self.MaxCount`))
    (`/Engine/EditorBlueprintResources/StandardMacros.IncrementInt` (`self.PalletCount`)
      (:`  `
        (set `self.CurrentCount` 0)))))

(fn `UserConstructionScript`)