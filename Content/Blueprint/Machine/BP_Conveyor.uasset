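; BP_Conveyor is a machine actor that carries parcels along its forward direction and can be selected by clicking.
; MoveArea overlaps add or remove parcels in CurrentParcels, toggle each one's EnterConveyor flag and fire OnConveyorStateChanged.
; Tick moves every tracked parcel by MoveSpeed scaled with delta time, setting location without sweep or physics.
; Clicking the Conveyor component passes the actor to BP_PlayerContoller through OnEquipmentSelected.
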(event `self.MoveArea.OnComponentBeginOverlap`
  (params (OverlappedComponent :type "PrimitiveComponent Object Reference") (OtherActor :type "Actor Object Reference") (OtherComp :type "PrimitiveComponent Object Reference") (OtherBodyIndex :type Integer) (bFromSweep :type Boolean) (SweepResult :type "HitResult Structure (by ref)"))
  (bind _currentparcels (`self.CurrentParcels`))
  ; Collision안으로 들어온 객체가 parcel이면 따로 저장
  (bind _asbp_parcel (cast `/Game/Blueprint/Parcel/BP_Parcel` OtherActor))
  (bind _returnvalue (`KismetArrayLibrary.Array_AddUnique` _currentparcels _asbp_parcel))
  (`self.OnConveyorStateChanged`)
  (set `/Game/Blueprint/Parcel/BP_Parcel.bEnterConveyor` true (`|GetArrayItem` _currentparcels _returnvalue)))

(event `self.MoveArea.OnComponentEndOverlap`
  (params (OverlappedComponent :type "PrimitiveComponent Object Reference") (OtherActor :type "Actor Object Reference") (OtherComp :type "PrimitiveComponent Object Reference") (OtherBodyIndex :type Integer))
  ; 나간 객체가 parcel이면 저장 해제
  (bind _asbp_parcel (cast `/Game/Blueprint/Parcel/BP_Parcel` OtherActor))
  (set `/Game/Blueprint/Parcel/BP_Parcel.bEnterConveyor` false _asbp_parcel)
  (`KismetArrayLibrary.Array_RemoveItem` (`self.CurrentParcels`) _asbp_parcel)
  (`self.OnConveyorStateChanged`))

(event `self.ReceiveTick`
  (params (DeltaSeconds :type "Float (single-precision)"))
  ; 컨베이어에 올라 왔다면, 앞으로 조금씩 전진
  (for _array_element (`self.CurrentParcels`)
    (`/Engine/EditorBlueprintResources/StandardMacros.IsValid` _array_element
      (:`Is Valid`
        (`self.K2_SetActorLocation` _array_element (+ (`self.K2_GetActorLocation` _array_element) (* DeltaSeconds (* (`self.MoveSpeed`) (`self.GetActorForwardVector`)))) false false)))))

(event `self.Conveyor.OnClicked`
  (params (TouchedComponent :type "PrimitiveComponent Object Reference") (ButtonPressed :type "Key Structure"))
  ; 클릭시 객체 정보 전달
  (bind _asbp_player_contoller (cast `/Game/Blueprint/Core/BP_PlayerContoller` (`GameplayStatics.GetPlayerController` 0)))
  (`/Game/Blueprint/Core/BP_PlayerContoller.OnEquipmentSelected` _asbp_player_contoller self)
  (`KismetSystemLibrary.PrintString` "전달 완료"))

(fn `UserConstructionScript`)