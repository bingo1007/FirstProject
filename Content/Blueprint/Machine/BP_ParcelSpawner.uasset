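; BP_ParcelSpawner spawns BP_Parcel actors at randomized short intervals along its SpawnDirection transform for the logistics system.
; It caches BP_LogisticsManager on BeginPlay, then runs a self-rescheduling timer that skips spawning in one SystemStatus state but keeps polling.
; Each parcel gets a manager-generated ID and label visibility, is counted as entering the system, and receives one of three random destinations.
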(event `ScheduleNextSpawn`
  ; 랜덤한 시간에 따라 Parcel 생성
  (`KismetSystemLibrary.K2_SetTimerDelegate` (delegate `SpawnParcel`) (`KismetMathLibrary.RandomFloatInRange` 1.0 2.0) :!label _label))

(event `self.ReceiveBeginPlay`
  ; 상태 체크를 위한 로지스틱스 매니저 캐싱
  (bind _returnvalue (`GameplayStatics.GetActorOfClass` "/Game/Blueprint/Core/BP_LogisticsManager.BP_LogisticsManager_C"))
  (bind _asbp_logistics_manager (cast `/Game/Blueprint/Core/BP_LogisticsManager` _returnvalue))
  (set `self.LogisticsManagerRef` _asbp_logistics_manager)
  (goto _label))

(event `SpawnParcel`
  (bind _logisticsmanagerref (`self.LogisticsManagerRef`))
  ; 현재 상태가 Running인지 확인. 맞다면 계속해서 박스 생성
  (`/Engine/EditorBlueprintResources/StandardMacros.IsValid` _logisticsmanagerref
    (:`Is Valid`
      (if (`|EnumInequality` (`/Game/Blueprint/Core/BP_LogisticsManager.SystemStatus` _logisticsmanagerref) "NewEnumerator2")
        ; 화살표 방향에 따라 박스 생성
        (bind _returnvalue (`|SpawnActorFromClass` "/Game/Blueprint/Parcel/BP_Parcel.BP_Parcel_C" (`SceneComponent.K2_GetComponentToWorld` (`self.SpawnDirection`)) "AlwaysSpawn" "MultiplyWithRoot" null null))
        ; Parcel ID 디스플레이 설정
        (set `/Game/Blueprint/Parcel/BP_Parcel.ParcelID` (`KismetTextLibrary.Conv_TextToString` (`/Game/Blueprint/Core/BP_LogisticsManager.GenerateParcelID` (`self.LogisticsManagerRef`))) _returnvalue)
        (`/Game/Blueprint/Parcel/BP_Parcel.UpdateParcelIDDisplay` _returnvalue)
        (`/Game/Blueprint/Parcel/BP_Parcel.SetParcelIDVisible` _returnvalue (`/Game/Blueprint/Core/BP_LogisticsManager.bShowParcelID` (`self.LogisticsManagerRef`)))
        ; 생성시 InSys값 +1
        (`/Game/Blueprint/Core/BP_LogisticsManager.ParcelEnteredSystem` (`self.LogisticsManagerRef`))
        ; 랜덤값에 따라 목적지도 랜덤으로 배정
        (switch `int` (`KismetMathLibrary.RandomIntegerInRange` 0 2)
          (:`0`
            (set `/Game/Blueprint/Parcel/BP_Parcel.Destination` "NewEnumerator0" _returnvalue))
          (:`1`
            (set `/Game/Blueprint/Parcel/BP_Parcel.Destination` "NewEnumerator1" _returnvalue))
          (:`2`
            (set `/Game/Blueprint/Parcel/BP_Parcel.Destination` "NewEnumerator2" _returnvalue)))
        (`self.ScheduleNextSpawn`)
        (else
          (`self.ScheduleNextSpawn`))))))

(fn `UserConstructionScript`)